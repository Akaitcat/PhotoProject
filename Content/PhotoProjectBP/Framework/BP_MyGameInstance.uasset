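; Game instance that manages page navigation and a pool of person media dialogs for the photo project UI.
; SwitchToPageView lazily creates and caches one widget per page type, hiding the current page before showing the next.
; Four BPW_MediaView widgets, each bound to its own media player, material and texture, cycle between cache and active lists.
; Showing a dialog that empties the cache recycles the oldest, keeping a spare available.
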(fn SwitchtoPageView
  (params (PageType :type BPE_ViewWidgetType%20Enum :default "NewEnumerator0"))
  (bind _pagetypemap (Variables|Default|GetPageTypeMap))
  (bind _pagewidgetmap (Variables|Default|GetPageWidgetMap))
  (bind (_value _returnvalue) (Utilities|Map|Find _pagetypemap PageType))
  (bind (_value_2 _returnvalue_2) (Utilities|Map|Find _pagewidgetmap PageType))
  (Utilities|FlowControl|Sequence
    (:then_0
      (if (not (Utilities|Map|Contains (Variables|Default|GetPageWidgetMap) PageType))
        (if _returnvalue
          (bind _returnvalue_3 (UserInterface|CreateWidget _value (Game|GetPlayerController 0)))
          (UserInterface|Viewport|AddtoViewport _returnvalue_3 0)
          (Class|BPISwitchablePage|SetVisible(Message) _returnvalue_3 false)
          (Utilities|Map|Add (Variables|Default|GetPageWidgetMap) PageType _returnvalue_3)
          (else
            (Development|PrintString (Utilities|String|Append "未找到页面类型:" (Utilities|String|ToString(Byte) PageType)))))))
    (:then_1
      (if _returnvalue_2
        (Utilities|IsValid (Variables|Default|GetCurrentPageWidget)
          (:Is%20Valid
            (Class|BPISwitchablePage|Hide(Message) (Variables|Default|GetCurrentPageWidget)))
          (:Is%20Not%20Valid
            _))
        (Class|BPISwitchablePage|Show(Message) _value_2)
        (Variables|Default|SetCurrentPageWidget _value_2)))))

(fn ShowMediaDialog
  (params (PersonData :type Person%20Data%20Object%20Reference) (Position :type Vector%202D%20Structure) (Owner :type BPW%20Loop%20View%20Object%20Reference))
  (bind _currentdialogviews (Variables|Default|GetCurrentDialogViews))
  (bind _cachedialogviews (Variables|Default|GetCacheDialogViews))
  (bind _cachedialogviews_2 (Variables|Default|GetCacheDialogViews))
  (bind _output (Utilities|Array|Get(acopy) _currentdialogviews))
  (bind _output_2 (Utilities|Array|Get(acopy) _cachedialogviews_2))
  (Utilities|FlowControl|Sequence
    (:then_0
      (if (<= (Utilities|Array|Length (Variables|Default|GetCacheDialogViews)) 0)
        (CallFunction|InitMediaView)))
    (:then_1
      (UserInterface|Viewport|AddtoViewport _output_2 1)
      (Default|InitData _output_2 PersonData Position Owner)
      (Utilities|Array|Add (Variables|Default|GetCurrentDialogViews) _output_2)
      (Utilities|Array|RemoveIndex _cachedialogviews)
      (if (<= (Utilities|Array|Length _cachedialogviews) 0)
        (Default|Recycle _output)
        (Utilities|Array|Add (Variables|Default|GetCacheDialogViews) _output)
        (Utilities|Array|RemoveIndex _currentdialogviews)))))

(fn InitMediaView
  (for _index (range 0 3)
    (bind _returnvalue (UserInterface|CreateWidget "/Game/PhotoProjectBP/UI/BPW_MediaView.BPW_MediaView_C" (Game|GetPlayerController 0) (Utilities|Select :Index _index :Option%200 "/Game/PhotoProjectBP/UI/MediaView/MediaPlayers/PersonMediaPlayer_1.PersonMediaPlayer_1" :Option%201 "/Game/PhotoProjectBP/UI/MediaView/MediaPlayers/PersonMediaPlayer_2.PersonMediaPlayer_2" :Option%202 "/Game/PhotoProjectBP/UI/MediaView/MediaPlayers/PersonMediaPlayer_3.PersonMediaPlayer_3" :Option%203 "/Game/PhotoProjectBP/UI/MediaView/MediaPlayers/PersonMediaPlayer_4.PersonMediaPlayer_4") (Utilities|Select :Index _index :Option%200 "/Game/PhotoProjectBP/UI/MediaView/MediaPlayerMaterials/MI_UI_PersonMediaMat_1.MI_UI_PersonMediaMat_1" :Option%201 "/Game/PhotoProjectBP/UI/MediaView/MediaPlayerMaterials/MI_UI_PersonMediaMat_2.MI_UI_PersonMediaMat_2" :Option%202 "/Game/PhotoProjectBP/UI/MediaView/MediaPlayerMaterials/MI_UI_PersonMediaMat_3.MI_UI_PersonMediaMat_3" :Option%203 "/Game/PhotoProjectBP/UI/MediaView/MediaPlayerMaterials/MI_UI_PersonMediaMat_4.MI_UI_PersonMediaMat_4") (Utilities|Select :Index _index :Option%200 "/Game/PhotoProjectBP/UI/MediaView/MediaPlayers/PersonMediaPlayer_Video_1.PersonMediaPlayer_Video_1" :Option%201 "/Game/PhotoProjectBP/UI/MediaView/MediaPlayers/PersonMediaPlayer_Video_2.PersonMediaPlayer_Video_2" :Option%202 "/Game/PhotoProjectBP/UI/MediaView/MediaPlayers/PersonMediaPlayer_Video_3.PersonMediaPlayer_Video_3" :Option%203 "/Game/PhotoProjectBP/UI/MediaView/MediaPlayers/PersonMediaPlayer_Video_4.PersonMediaPlayer_Video_4")))
    (Utilities|Array|Add (Variables|Default|GetCacheDialogViews) _returnvalue)))

(fn RecycleMediaDialog
  (params (MediaDialog :type BPW%20Media%20View%20Object%20Reference))
  (Utilities|Array|Add (Variables|Default|GetCacheDialogViews) MediaDialog)
  (Default|Recycle MediaDialog))

(fn ClearMediaDialog
  (bind _currentdialogviews (Variables|Default|GetCurrentDialogViews))
  (for _array_element _currentdialogviews
    (CallFunction|RecycleMediaDialog _array_element))
  (Utilities|Array|Clear _currentdialogviews))

(fn IsPersonShow
  (params (Person :type Person%20Data%20Object%20Reference))
  (for _array_element (Variables|Default|GetCurrentDialogViews)
    (if (== (Variables|/Game/PhotoProjectBP/UI/BPW_MediaView.BPW_MediaView_C|GetPersonData _array_element) Person)
      (return true)))
  (return false))